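; BP_Nuke runs the nuke launch countdown and ends the game once the nuke is triggered.
; On BeginPlay it starts a one-shot timer, timed by the Rules on BP_COLDefenceInstance, that calls SendNuke when it expires.
; It also binds EndTheGame to the NukeTriggered event, which pauses the game after a short delay without checking IsNukeSent.
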(event Custom|EndTheGame
  (params (bIsNukeSent :type Boolean))
  (Utilities|FlowControl|Delay 1e+01)
  (Game|SetGamePaused true))

(event Custom|Nuuuuke
  (Class|NukeBase|SendNuke))

(event EventBeginPlay
  (EventDispatchers|BindEventtoNukeTriggered (delegate Custom|EndTheGame))
  (bind _asbp_coldefence_instance (Utilities|Casting|CastToBP_COLDefenceInstance (Game|GetGameInstance)))
  (bind _returnvalue (Utilities|Time|SetTimerbyEvent (delegate Custom|Nuuuuke) (.nukelaunchtimeinseconds (Variables|/Script/COLDefence.COLDefenceInstance|GetRules _asbp_coldefence_instance))))
  (Variables|Default|SetNukeTimerHandle _returnvalue))

(event Collision|EventActorBeginOverlap
  (params (OtherActor :type Actor%20Object%20Reference)))

(event EventTick
  (params (DeltaSeconds :type Float%20%28single-precision%29)))

(fn ConstructionScript)