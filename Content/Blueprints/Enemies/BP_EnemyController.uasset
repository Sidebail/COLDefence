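; AI controller for enemies that runs a behavior tree and tracks a shootable target through blackboard keys.
; On begin play it briefly waits, then stores the game instance's Nuke as the nuke target.
; Pawn sensing locks the first seen pawn that passes CanShootTarget as the current target.
; Tick clears that target once it becomes invalid or moves beyond sight radius, letting sensing pick another.
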(event OnSeePawn(SensingComponent)
  (params (Pawn :type Pawn%20Object%20Reference))
  (bind _blackboard (Variables|Default|GetBlackboard))
  (bind _returnvalue (Class|EnemyController|CanShootTarget Pawn))
  (if (and _returnvalue (not (ScalableFloat|GetValueasBool (Variables|Default|GetBlackboard) (Variables|Default|GetBBKey_IsProperTargetFound))))
    (AI|Components|Blackboard|SetValueasBool _blackboard (Variables|Default|GetBBKey_IsProperTargetFound) true)
    (AI|Components|Blackboard|SetValueasObject _blackboard (Variables|Default|GetBBKey_CurrentTarget) Pawn)))

(event EventTick
  (params (DeltaSeconds :type Float%20%28single-precision%29))
  (bind _blackboard (Variables|Default|GetBlackboard))
  (bind _bbkey_currenttarget (Variables|Default|GetBBKey_CurrentTarget))
  (bind _blackboard_2 (Variables|Default|GetBlackboard))
  (bind _returnvalue (AI|Components|Blackboard|GetValueasObject _blackboard _bbkey_currenttarget))
  (if (ScalableFloat|GetValueasBool (Variables|Default|GetBlackboard) (Variables|Default|GetBBKey_IsProperTargetFound))
    (Utilities|IsValid _returnvalue
      (:Is%20Valid
        (if (> (Transformation|GetDistanceTo (Pawn|GetControlledPawn) (.AsActor (Utilities|Casting|CastToActor _returnvalue))) (Variables|/Script/AIModule.PawnSensingComponent|GetSightRadius (Variables|Default|GetSensingComponent)))
          (AI|Components|Blackboard|SetValueasBool _blackboard_2 (Variables|Default|GetBBKey_IsProperTargetFound) false :!label _label)
          (AI|Components|Blackboard|SetValueasObject _blackboard_2 (Variables|Default|GetBBKey_CurrentTarget) 0)))
      (:Is%20Not%20Valid
        (goto _label)))))

(event EventBeginPlay
  (AI|RunBehaviorTree (Variables|Default|GetBehaviorTree))
  (Utilities|FlowControl|Delay 0.2)
  (AI|Components|Blackboard|SetValueasObject (Variables|Default|GetBlackboard) (Variables|Default|GetBBKey_NukeTarget) (Variables|/Script/COLDefence.COLDefenceInstance|GetNuke (.AsBP%20COLDefence%20Instance (Utilities|Casting|CastToBP_COLDefenceInstance (Game|GetGameInstance))))))

(fn ConstructionScript)